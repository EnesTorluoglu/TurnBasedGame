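; BP_MapWar is a campaign map "goable" that brings up the war UI when a map group reaches it.
; Its group overlap event runs the parent handling, then creates a WBP_War widget and adds it to the viewport.
; The construction script only calls the parent, and the BeginPlay, Tick and actor overlap events are disabled placeholders.
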(event EventBeginPlay
  (|CallParentFunction) ; This node is disabled and will not be called.\nDrag off pins to build functionality.
)

(event Collision|EventActorBeginOverlap
  (params (OtherActor :type Actor%20Object%20Reference))
  (|CallParentFunction OtherActor) ; This node is disabled and will not be called.\nDrag off pins to build functionality.
)

(event EventTick
  (params (DeltaSeconds :type Float%20%28single-precision%29))
  (|CallParentFunction DeltaSeconds) ; This node is disabled and will not be called.\nDrag off pins to build functionality.
)

(event EventGroupBeginOverlap
  (params (mapGroup :type Map%20Groups%20Object%20Reference))
  (|CallParentFunction mapGroup)
  (bind _returnvalue (UserInterface|CreateWidget "/Game/BaseMode/Widget/CampaignMap/WBP_War.WBP_War_C"))
  (UserInterface|Viewport|AddtoViewport _returnvalue 0))

(fn ConstructionScript
  (|CallParentFunction))