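; BP_City is a city actor on the campaign map that map groups can travel to and enter.
; Hovering the cursor over its mesh toggles custom depth rendering as a highlight.
; When a BP_MapGroups heading for this city overlaps its box, the city messages the group to stop and notifies the player's view target.
; It then shows a WBP_City widget with the city name and pauses the game after a short delay.
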(event OnBeginCursorOver(StaticMesh)
  (params (TouchedComponent :type Primitive%20Component%20Object%20Reference))
  (Rendering|SetRenderCustomDepth TouchedComponent true))

(event OnEndCursorOver(StaticMesh)
  (params (TouchedComponent :type Primitive%20Component%20Object%20Reference))
  (Rendering|SetRenderCustomDepth TouchedComponent false))

(event OnComponentBeginOverlap(Box)
  (params (OverlappedComponent :type Primitive%20Component%20Object%20Reference) (OtherActor :type Actor%20Object%20Reference) (OtherComp :type Primitive%20Component%20Object%20Reference) (OtherBodyIndex :type Integer) (bFromSweep :type Boolean) (SweepResult :type Hit%20Result%20Structure%20%28by%20ref%29))
  (if (== "/Game/BaseMode/Blueprints/CampaignMap/BP_MapGroups.BP_MapGroups_C" (Utilities|GetClass OtherActor))
    (bind _asbp_map_groups (Utilities|Casting|CastToBP_MapGroups OtherActor))
    (if (and (== self (Variables|/Game/BaseMode/Blueprints/CampaignMap/BP_MapGroups.BP_MapGroups_C|GetCityToGo _asbp_map_groups)) (Variables|/Game/BaseMode/Blueprints/CampaignMap/BP_MapGroups.BP_MapGroups_C|GetIsGoingToCity _asbp_map_groups))
      (Class|BPICampaignInteractable|StopMovement(Message) OtherActor)
      (Class|BPICampaignInteractable|GotoCity(Message) (Pawn|GetViewTarget (Game|GetPlayerController 0)) self)
      (bind _returnvalue (UserInterface|CreateWidget "/Game/BaseMode/Widget/WBP_City.WBP_City_C"))
      (Default|SetCityName _returnvalue (Variables|Default|GetCityName))
      (UserInterface|Viewport|AddtoViewport _returnvalue 0)
      (Utilities|FlowControl|Delay 0.2)
      (Game|SetGamePaused true))))

(event EventBeginPlay)

(event Collision|EventActorBeginOverlap
  (params (OtherActor :type Actor%20Object%20Reference)))

(event EventTick
  (params (DeltaSeconds :type Float%20%28single-precision%29)))

(fn ConstructionScript)