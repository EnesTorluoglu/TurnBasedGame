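; Player controller for the campaign map that handles camera zoom, unit selection and move orders.
; Left click deselects the previous unit, then traces a dedicated channel under the cursor and selects the hit actor through message calls.
; Holding right mouse opens a Tick gate that continuously sends the cursor's world location to the selected unit.
; The mouse wheel sets the campaign camera's spring arm length within clamped limits.
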(event EventBeginPlay
  (Input|SetInputModeGameandUI self 0 "LockAlways" false)
  (bind _asbp_campaign_camera (Utilities|Casting|CastToBP_CampaignCamera (Pawn|GetViewTarget)))
  (Variables|Default|SetCampaignCamera _asbp_campaign_camera))

(event EventTick
  (params (DeltaSeconds :type Float%20%28single-precision%29))
  (Utilities|FlowControl|Gate true
    (:Exit
      (Class|BPICampaignInteractable|MovetoCursor(Message) (Variables|Default|GetLastSelectedComp) (.location (.HitResult (Game|Player|GetHitResultUnderCursorbyChannel (Game|GetPlayerController 0) "TraceTypeQuery1" true)))))))

(event Input|MouseEvents|MouseWheelAxis
  (params (AxisValue :type Float%20%28single-precision%29))
  ;[1 1 1] Zoom In/Out
  (if (!= AxisValue 0.0)
    (bind _output_get (Variables|Default|SetZoomFactor (Math|Float|Clamp(Float) (+ (* AxisValue -1.0) (Variables|Default|GetZoomFactor)) 2.0 1e+01)))
    (Variables|/Script/Engine.SpringArmComponent|SetTargetArmLength (Variables|/Game/BaseMode/Blueprints/CampaignMap/Fundamental/BP_CampaignCamera.BP_CampaignCamera_C|GetSpringArm (Variables|Default|GetCampaignCamera)) (* _output_get 5e+02))))

(event Input|MouseEvents|LeftMouseButton
  (params (Key :type Key%20Structure :default "None"))
  (bind _self self)
  (bind _hitresult (Game|Player|GetHitResultUnderCursorbyChannel _self "TraceTypeQuery7" true))
  (:Pressed
    (Class|BPICampaignInteractable|DeselectUnit(Message) (Variables|Default|GetLastSelectedComp))
    (if (.bblockinghit _hitresult)
      (bind _output_get (Variables|Default|SetLastSelectedComp (.hitactor _hitresult)))
      (Class|BPICampaignInteractable|SelectUnit(Message) _output_get))))

(event Input|MouseEvents|RightMouseButton
  (params (Key :type Key%20Structure :default "None"))
  (:Pressed
    (Utilities|FlowControl|Gate true) ; enters at Open
  )
  (:Released
    (Utilities|FlowControl|Gate true) ; enters at Close
  ))

(fn ConstructionScript)