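; BP_MapGroups is a selectable, AI-moved unit group on the campaign map.
; On BeginPlay it caches every BP_MapCharacter in the level, with no filtering by group.
; Selecting or deselecting toggles custom depth on those characters' meshes for highlighting.
; When selected, a move order restarts the group's own AI move, spawns a cursor effect at the destination and forwards that location to each cached character.
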(event EventBeginPlay
  (bind _outactors (Actor|GetAllActorsOfClass "/Game/BaseMode/Blueprints/CampaignMap/BP_MapCharacter.BP_MapCharacter_C"))
  (Variables|Default|SetMapCharacters _outactors))

(event Collision|EventActorBeginOverlap
  (params (OtherActor :type Actor%20Object%20Reference)))

(event EventTick
  (params (DeltaSeconds :type Float%20%28single-precision%29)))

(event EventSelectUnit
  ;[1 1 1] Select/Deselect(Highlight) Units In the Group
  (Variables|Default|SetIsSelected true)
  (for _array_element (Variables|Default|GetMapCharacters)
    (Rendering|SetRenderCustomDepth (Variables|/Script/Engine.Character|GetMesh _array_element) true)))

(event EventDeselectUnit
  ;[1 1 1] Select/Deselect(Highlight) Units In the Group
  (Variables|Default|SetIsSelected false)
  (for _array_element (Variables|Default|GetMapCharacters)
    (Rendering|SetRenderCustomDepth (Variables|/Script/Engine.Character|GetMesh _array_element) false)))

(event EventMovetoCursor
  (params (LocationToGo :type Vector :default "0, 0, 0"))
  (bind _self self)
  (bind _returnvalue (AI|GetAIController _self))
  (if (Variables|Default|GetIsSelected)
    (AI|Navigation|StopMovement _returnvalue)
    (AI|AIMoveTo _returnvalue LocationToGo 0 -1.0 "Default" "Default" true true
      (:then
        (Niagara|SpawnSystematLocation "/Game/BaseMode/Cursor/FX_Cursor.FX_Cursor" LocationToGo)
        (for _array_element (Variables|Default|GetMapCharacters)
          (Class|BPICampaignInteractable|MovetoCursor(Message) _array_element LocationToGo))))))

(fn ConstructionScript)