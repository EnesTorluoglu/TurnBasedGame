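; BP_Company is a selectable company unit for the campaign map, filed among experimental, outdated assets.
; Select and deselect events set the selection flag and toggle custom depth rendering on both of its meshes for highlighting.
; When selected, a move command stops current AI movement, issues AIMoveTo toward the given location and immediately spawns a cursor effect there.
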(event EventSelectUnit
  ;[1 1 1] Select/Deselect Unit
  (Variables|Default|SetIsSelected true)
  (Rendering|SetRenderCustomDepth (Variables|Default|GetSkeletalMesh) true)
  (Rendering|SetRenderCustomDepth (Variables|Character|GetMesh) true))

(event EventDeselectUnit
  ;[1 1 1] Select/Deselect Unit
  (Variables|Default|SetIsSelected false)
  (Rendering|SetRenderCustomDepth (Variables|Default|GetSkeletalMesh) false)
  (Rendering|SetRenderCustomDepth (Variables|Character|GetMesh) false))

(event EventMovetoCursor
  (params (LocationToGo :type Vector :default "0, 0, 0"))
  (bind _self self)
  (bind _returnvalue (AI|GetAIController _self))
  ;[1 1 1] Move To Clicked Location
  (if (Variables|Default|GetIsSelected)
    (AI|Navigation|StopMovement _returnvalue)
    (AI|AIMoveTo _returnvalue LocationToGo 0 -1.0 "Default" "Default" true true
      (:then
        (Niagara|SpawnSystematLocation "/Game/BaseMode/Cursor/FX_Cursor.FX_Cursor" LocationToGo)))))

(fn ConstructionScript)