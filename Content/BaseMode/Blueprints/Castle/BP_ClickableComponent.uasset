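; BP_ClickableComponent is an actor component in the Castle folder that highlights its owning actor while the mouse cursor is over it.
; On BeginPlay it caches the owner's skeletal mesh and, if one exists, binds to the owner's begin and end cursor-over events.
; Those handlers toggle Render Custom Depth on the mesh, and the hover handler also prints a debug "Hello".
; Despite the name, it contains no click handling.
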(event Custom|OnMouseHover
  (params (TouchedActor :type Actor%20Object%20Reference))
  (Development|PrintString "Hello")
  (Rendering|SetRenderCustomDepth (Variables|Default|GetSkeletalMeshRef) true))

(event Custom|OnMouseHoverEnd
  (params (TouchedActor :type Actor%20Object%20Reference))
  (Rendering|SetRenderCustomDepth (Variables|Default|GetSkeletalMeshRef) false))

(event EventBeginPlay
  (bind _returnvalue (Components|GetOwner))
  (bind _returnvalue_2 (Actor|GetComponentbyClass _returnvalue "/Script/Engine.SkeletalMeshComponent"))
  (Utilities|IsValid _returnvalue_2
    (:Is%20Valid
      (Variables|Default|SetSkeletalMeshRef _returnvalue_2)
      (EventDispatchers|BindEventtoOnBeginCursorOver _returnvalue (delegate Custom|OnMouseHover))
      (EventDispatchers|BindEventtoOnEndCursorOver _returnvalue (delegate Custom|OnMouseHoverEnd)))))