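; BP_CastleController is the player controller for the castle mode, handling camera zoom and pause menu input.
; On BeginPlay it locks the mouse in game-and-UI mode and caches the BP_CastleCamera view target.
; The mouse wheel drives a clamped zoom factor into the camera's spring arm length, with setters toggling zoom and camera movement.
; The P key alternates open and close pause menu messages to the HUD via a FlipFlop.
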(event EventBeginPlay
  (Input|SetInputModeGameandUI self 0 "LockAlways" false)
  (bind _asbp_castle_camera (Utilities|Casting|CastToBP_CastleCamera (Pawn|GetViewTarget)))
  (Variables|Default|SetBPCamera _asbp_castle_camera))

(event EventSetIsZoomable
  (params (IsZoomable :type Boolean))
  (Variables|Default|SetIsZoomable IsZoomable))

(event EventSetIsCameraMovable
  (params (IsCameraMovable :type Boolean))
  (Variables|/Game/BaseMode/Blueprints/Castle/BP_CastleCamera.BP_CastleCamera_C|SetIsMovable (Variables|Default|GetBPCamera) IsCameraMovable))

(event Input|MouseEvents|MouseWheelAxis
  (params (AxisValue :type Float%20%28single-precision%29))
  (if (and (!= AxisValue 0.0) (Variables|Default|GetIsZoomable))
    (bind _output_get (Variables|Default|SetZoomFactor (Math|Float|Clamp(Float) (+ (* AxisValue -1.0) (Variables|Default|GetZoomFactor)) 0.0 2e+01)))
    (Variables|/Script/Engine.SpringArmComponent|SetTargetArmLength (Variables|/Game/BaseMode/Blueprints/Castle/BP_CastleCamera.BP_CastleCamera_C|GetSpringArm (Variables|Default|GetBPCamera)) (* _output_get 1e+02))))

(event Input|KeyboardEvents|P
  (params (Key :type Key%20Structure :default "None"))
  (bind _returnvalue (HUD|GetHUD))
  (:Pressed
    (Utilities|FlowControl|FlipFlop
      (:A
        (Class|BPIUICommunication|OpenPauseMenu(Message) _returnvalue))
      (:B
        (Class|BPIUICommunication|ClosePauseMenu(Message) _returnvalue)))))

(fn ConstructionScript)