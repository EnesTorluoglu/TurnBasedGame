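; BP_HUD_Castle is the HUD for the castle base mode, managing the main base UI and the pause menu.
; On BeginPlay it creates WBP_BaseUI and adds it to the viewport.
; OpenPauseMenu collapses the base UI, creates a new WBP_PauseMenu and pauses the game.
; ClosePauseMenu removes that menu, unpauses and shows the base UI again.
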(event EventBeginPlay
  (bind _returnvalue (UserInterface|CreateWidget "/Game/BaseMode/Widget/Castle/WBP_BaseUI.WBP_BaseUI_C"))
  (bind _output_get (Variables|Default|SetBaseUI _returnvalue))
  (UserInterface|Viewport|AddtoViewport _output_get 0))

(event EventOpenPauseMenu
  (Widget|SetVisibility (Variables|Default|GetBaseUI) "Collapsed")
  (bind _returnvalue (UserInterface|CreateWidget "/Game/BaseMode/Widget/WBP_PauseMenu.WBP_PauseMenu_C"))
  (bind _output_get (Variables|Default|SetPauseMenu _returnvalue))
  (UserInterface|Viewport|AddtoViewport _output_get 0)
  (Game|SetGamePaused true))

(event EventClosePauseMenu
  (Widget|RemovefromParent (Variables|Default|GetPauseMenu))
  (Game|SetGamePaused false)
  (Widget|SetVisibility (Variables|Default|GetBaseUI) "Visible"))

(fn ConstructionScript)