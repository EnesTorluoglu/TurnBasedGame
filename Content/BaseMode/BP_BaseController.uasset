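; BP_BaseController is a player controller that drives mouse-wheel zoom for a BP_MapCamera view target.
; On begin play it sets game-and-UI input with the mouse always locked and caches the view target as the map camera.
; Mouse wheel input adjusts a clamped, inverted zoom factor, which is scaled to set the camera's spring arm length.
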(event EventBeginPlay
  (Input|SetInputModeGameandUI self 0 "LockAlways" false)
  (bind _asbp_camera (Utilities|Casting|CastToBP_MapCamera (Pawn|GetViewTarget)))
  (Variables|Default|SetBPCamera _asbp_camera))

(event Input|MouseEvents|MouseWheelAxis
  (params (AxisValue :type Float%20%28single-precision%29))
  (bind _output_get (Variables|Default|SetZoomFactor (Math|Float|Clamp(Float) (+ (* AxisValue -1.0) (Variables|Default|GetZoomFactor)) 0.0 1e+01)))
  (Variables|/Script/Engine.SpringArmComponent|SetTargetArmLength (Variables|/Game/BaseMode/BP_MapCamera.BP_MapCamera_C|GetSpringArm (Variables|Default|GetBPCamera)) (* _output_get 6.0)))

(fn ConstructionScript)